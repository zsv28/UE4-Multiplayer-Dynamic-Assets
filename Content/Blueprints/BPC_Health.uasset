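; BPC_Health is a health component Blueprint that tracks current health against a maximum.
; It starts at MaxHealth on BeginPlay, and TakesDamage subtracts damage, clamps the result between zero and the maximum, and returns it.
; GetHealth and IsDead expose the state, while a RepNotify on Health only prints the new value.
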(event EventBeginPlay
  (Variables|Default|SetHealth (Variables|Default|GetMaxHealth)))

(event EventTick
  (params (DeltaSeconds :type Float%20%28single-precision%29)))

(fn GetHealth
  (return (Variables|Default|GetHealth)))

(fn IsDead
  (return (<= (Variables|Default|GetHealth) 0.0)))

(fn TakesDamage
  (params (Damage :type Float%20%28single-precision%29))
  (bind _output_get (Variables|Default|SetHealth (Math|Float|Clamp(Float) (- (Variables|Default|GetHealth) Damage) 0.0 (Variables|Default|GetMaxHealth))))
  (return _output_get))

(fn OnRepHealth
  (Development|PrintString (Utilities|String|ToString(Float) (Variables|Default|GetHealth))))