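; Multiplayer game mode that splits joining players into two teams.
; On PostLogin it casts the controller to BP_MultiplayerPlayerController, puts it on the smaller team (Team 1 on a tie), sets its TeamID and stores it in that team's array.
; On logout it removes the controller from the array matching its TeamID.
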(event EventBeginPlay)

(event EventTick
  (params (DeltaSeconds :type Float%20%28single-precision%29)))

(event EventPostLogin
  (params (NewPlayer :type Player%20Controller%20Object%20Reference))
  (bind _asbp_multiplayer_player_controller (Utilities|Casting|CastToBP_MultiplayerPlayerController NewPlayer)
    (:then
      (if (< (Utilities|Array|Length (Variables|Default|GetTeam%202)) (Utilities|Array|Length (Variables|Default|GetTeam%201)))
        (Default|SetTeamID _asbp_multiplayer_player_controller 2)
        (Utilities|Array|Add (Variables|Default|GetTeam%202) _asbp_multiplayer_player_controller)
        (else
          (Default|SetTeamID _asbp_multiplayer_player_controller 1)
          (Utilities|Array|Add (Variables|Default|GetTeam%201) _asbp_multiplayer_player_controller))))
    (:CastFailed
      (Development|PrintString "Post login error"))))

(event EventOnLogout
  (params (ExitingController :type Controller%20Object%20Reference))
  (bind _team_1 (Variables|Default|GetTeam%201))
  (bind _team_2 (Variables|Default|GetTeam%202))
  (bind _asbp_multiplayer_player_controller (Utilities|Casting|CastToBP_MultiplayerPlayerController ExitingController))
  (if (== (Variables|/Game/Blueprints/BP_MultiplayerPlayerController.BP_MultiplayerPlayerController_C|GetTeamID _asbp_multiplayer_player_controller) 1)
    (Utilities|Array|RemoveIndex _team_1 (Utilities|Array|FindItem _team_1 _asbp_multiplayer_player_controller))
    (elif (== (Variables|/Game/Blueprints/BP_MultiplayerPlayerController.BP_MultiplayerPlayerController_C|GetTeamID _asbp_multiplayer_player_controller) 2)
      (Utilities|Array|RemoveIndex _team_2 (Utilities|Array|FindItem _team_2 _asbp_multiplayer_player_controller)))))

(fn ConstructionScript)