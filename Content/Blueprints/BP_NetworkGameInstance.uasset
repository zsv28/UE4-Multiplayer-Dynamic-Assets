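; BP_NetworkGameInstance is a Game Instance that handles LAN multiplayer session hosting and joining.
; CreateGame creates a 16-slot LAN session and opens Testlvl as a listen server.
; JoinToGame searches LAN sessions and attempts to join every result in a loop, while GetGames is an empty stub whose logic moved to the wbp_slot widget.
; Session failures and network or travel errors are printed to screen.
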(event Custom|CreateGame
  ;[1 0.9743 0.3585] Create Game
  (|Session (Game|GetPlayerController 0) 16 true
    (:OnSuccess
      (Game|OpenLevel(byName) "Testlvl" true "?listen"))
    (:OnFailure
      (Development|PrintString "Game creation error!" true true "(R=1.000000,G=0.000000,B=0.000000,A=1.000000)"))))

(event Custom|GetGames
  ;[0.1302 0.1302 0.1302] Moved the logic to the widget wbp_slot
  ;;[0.578 0.524 1] Get Game
)

(event Custom|JoinToGame
  (bind _returnvalue (Game|GetPlayerController 0))
  ;[0.4891 1 0.3203] Join To Game
  (bind _results (|FindSessions _returnvalue 20 true)
    (:OnSuccess
      (for _array_element _results
        (|JoinSession _returnvalue _array_element
          (:OnFailure
            (Development|PrintString "Join to game error!")))))
    (:OnFailure
      (Development|PrintString "Game searching error!" true true "(R=0.729167,G=0.006447,B=0.000000,A=1.000000)"))))

(event EventHandleNetworkError
  (params (FailureType :type ENetworkFailure%20Enum :default "NetDriverAlreadyExists") (bIsServer :type Boolean))
  ;[1 0.228 0.2081] Errors
  (Development|PrintString (Utilities|String|Append "Network error: " (Utilities|String|EnumtoString FailureType) " on server? " (Utilities|String|ToString(Boolean) bIsServer))))

(event EventHandleTravelError
  (params (FailureType :type ETravelFailure%20Enum :default "NoLevel"))
  ;[1 0.228 0.2081] Errors
  (Development|PrintString (Utilities|String|Append "Network travel error: " (Utilities|String|EnumtoString FailureType))))