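; BP_Projectile is a multiplayer projectile that damages player pawns and explodes on impact.
; The server moves it forward each tick by setting its location without sweep and handles sphere overlaps.
; Overlaps ignore the owner and other projectiles; any other hit multicasts an explosion effect and disables further overlaps, with damage only for BP_MultiplayerPawn.
; A hit or lifetime timer expiry destroys the actor after a short delay.
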(event OnComponentBeginOverlap(Sphere)
  (params (OverlappedComponent :type Primitive%20Component%20Object%20Reference) (OtherActor :type Actor%20Object%20Reference) (OtherComp :type Primitive%20Component%20Object%20Reference) (OtherBodyIndex :type Integer) (bFromSweep :type Boolean) (SweepResult :type Hit%20Result%20Structure%20%28by%20ref%29))
  (if (Networking|IsServer)
    (CallFunction|ServerCollision OtherActor (Transformation|GetActorLocation))))

(event Custom|LifeEnded
  (CallFunction|ServerLifeEnded))

(event Custom|Server_LifeEnded
  (Utilities|FlowControl|Delay 0.2)
  (Actor|DestroyActor))

(event Custom|Server_Move
  (params (Delta%20Time :type Float%20%28single-precision%29))
  (Transformation|SetActorLocation (+ (Transformation|GetActorLocation) (* (Transformation|GetActorForwardVector) (* Delta%20Time (Variables|Default|GetSpeed)))) false false))

(event Custom|Server%20Collision
  (params (OtherActor :type Actor%20Object%20Reference) (Location :type Vector))
  (if (!= OtherActor (Components|GetOwner))
    (bind _asbp_multiplayer_pawn (Utilities|Casting|CastToBP_MultiplayerPawn OtherActor)
      (:then
        (Default|TakeDamage _asbp_multiplayer_pawn (Variables|Default|GetDamage)))
      (:CastFailed
        (Utilities|Casting|CastToBP_Projectile OtherActor
          (:CastFailed
            _))))
    (CallFunction|MulticastHirEffect Location)
    (Variables|/Script/Engine.PrimitiveComponent|SetbGenerateOverlapEvents (Variables|Default|GetSphere) false)
    (CallFunction|ServerLifeEnded)))

(event Custom|SpawnHitEffects
  (params (Location :type Vector))
  (Effects|SpawnEmitteratLocation "/Game/StarterContent/Particles/P_Explosion.P_Explosion" Location))

(event Custom|Multicast_HirEffect
  (params (Hit%20Location :type Vector))
  (CallFunction|SpawnHitEffects Hit%20Location))

(event EventBeginPlay
  (Utilities|Time|SetTimerbyEvent (delegate Custom|LifeEnded) (Variables|Default|GetTTL)))

(event EventTick
  (params (DeltaSeconds :type Float%20%28single-precision%29))
  (if (Networking|IsServer)
    (CallFunction|ServerMove DeltaSeconds)))

(fn ConstructionScript)